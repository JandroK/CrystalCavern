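; BP_CannonManager lets the cannons in its CannonList fire in turn at a timed interval.
; From BeginPlay, a looping Delay of TimeBetweenShoots sets CanShoot on the BP_Cannon at the current index.
; The IsValidIndex1 helper supplies the next index, and the index wraps to zero when that check fails.
; A failed cast to BP_Cannon ends the loop.
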(event `self.ReceiveBeginPlay`
  (`KismetSystemLibrary.Delay` (`self.TimeBetweenShoots`) :!label _label)
  (bind _asbp_cannon (cast `/Game/BluePrints/Actors/BP_Cannon` (`|GetArrayItem` (`self.CannonList`) (`self.Index`))))
  (set `/Game/BluePrints/Actors/BP_Cannon.CanShoot` true _asbp_cannon)
  (bind _new_index (`/Game/BluePrints/Libraries/CC_MacroLibrary.Is Valid Index +1` (`self.CannonList`) (`self.Index`))
    (:`True`
      (set `self.Index` _new_index)
      (goto _label))
    (:`False`
      (set `self.Index` 0)
      (goto _label))))

(fn `UserConstructionScript`)