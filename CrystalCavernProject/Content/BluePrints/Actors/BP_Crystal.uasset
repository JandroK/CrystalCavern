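; BP_Crystal is a collectible crystal actor that the player picks up by overlapping it.
; On first player overlap it plays a pickup sound and runs a timeline that pulls it toward just above the player pawn while shrinking it and fading its point light.
; It lerps from transform and light values cached on BeginPlay, then increments the crystal count on the W_HUD widget and destroys itself.
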(event `self.ReceiveBeginPlay`
  (`self.StartValues`))

(event `self.ReceiveActorBeginOverlap`
  (params (OtherActor :type "Actor Object Reference"))
  (`/Game/BluePrints/Libraries/CC_MacroLibrary.IsPlayer` OtherActor
    (:`Is Player`
      (`/Engine/EditorBlueprintResources/StandardMacros.DoOnce` false
        (:`Completed`
          (`GameplayStatics.PlaySoundAtLocation` "/Game/Sounds/PickUp_Crystal_Cue.PickUp_Crystal_Cue" (`self.K2_GetActorLocation`) (struct) 1.0 1.0 0.0 null null null null)
          (bind (_direction _linearvalue _light_intensity) (`Timeline|BlendBetweenVectors`)
            (:`Update`
              (`self.Blend Move To Player Pawn` _linearvalue)
              (`self.Scale To 0` _linearvalue)
              (`self.Adjust Light Intensity` _light_intensity))
            (:`Finished`
              (`self.Update UI`)
              (`self.K2_DestroyActor`))))))))

(fn `Adjust Light Intensity`
  (params (Alpha :type "Float (double-precision)"))
  (`LightComponent.SetIntensity` (`self.PointLight`) (`KismetMathLibrary.Lerp` (`self.StartLightIntensity`) 0.0 Alpha)))

(fn `Blend Move To Player Pawn`
  (params (Alpha :type "Float (single-precision)"))
  (`self.K2_SetActorLocation` (`KismetMathLibrary.VLerp` (`self.StartPos`) (+ (`self.K2_GetActorLocation` (`GameplayStatics.GetPlayerPawn` 0)) (0.0 0.0 50.0)) Alpha)))

(fn `Scale To 0`
  (params (Alpha :type "Float (single-precision)"))
  (`self.SetActorScale3D` (`KismetMathLibrary.VLerp` (`self.StartScale`) (0.0 0.0 0.0) Alpha)))

(fn `StartValues`
  (set `self.StartPos` (`self.K2_GetActorLocation`))
  (set `self.StartScale` (`self.GetActorScale3D`))
  (set `self.StartLightIntensity` (`LightComponentBase.Intensity` (`self.PointLight`))))

(fn `Update UI`
  (bind _foundwidgets (`WidgetBlueprintLibrary.GetAllWidgetsOfClass` "/Game/UI/W_HUD.W_HUD_C"))
  (`/Game/UI/W_HUD.Increment current crystals` (`|GetArrayItem` _foundwidgets)))

(fn `UserConstructionScript`)