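; BP_WinVolume is a trigger volume that completes the level when the player overlaps it and no BP_Crystal actors remain.
; After a camera fade, it overwrites the save slot with a fresh BP_SaveGame whose Continue flag is false.
; It then opens the next level in the LevelNames array, looping to the first after the last.
; A debug G key completes the level immediately, skipping the checks and fade.
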(event `Key|G`
  (params (Key :type "Key Structure"))
  ;[1 0.8093 0.1808] Debug Mode (Insta Next Level)
  (:`Pressed`
    (`self.Completed Level`)))

(event `self.ReceiveActorBeginOverlap`
  (params (OtherActor :type "Actor Object Reference"))
  (`/Game/BluePrints/Libraries/CC_MacroLibrary.IsPlayer` OtherActor
    (:`Is Player`
      (if (`self.None Crystal Remaining`)
        (`/Game/BluePrints/Libraries/CC_MacroLibrary.Start Camera Fade` 1.0
          (:`Completed`
            (`self.Completed Level`)))))))

(fn `Completed Level`
  (`self.Set ContinueGame to False`)
  (if (`self.Current Is Last Level`)
    (`self.Restart Game`)
    (else
      (`GameplayStatics.OpenLevel` (`self.Get Next Level Name`)))))

(fn `Current Is Last Level`
  (returns (Value :type Boolean))
  (return (>= (+ (`self.Get Current Level Index`) 1) (`KismetArrayLibrary.Array_Length` (`self.LevelNames`)))))

(fn `Get Current Level Index`
  (returns (Output :type Integer))
  (bind _returnvalue (`GameplayStatics.GetCurrentLevelName` true))
  (return (`KismetArrayLibrary.Array_Find` (`self.LevelNames`) _returnvalue)))

(fn `Get Next Level Name`
  (returns (Name :type Name))
  (return (`KismetStringLibrary.Conv_StringToName` (`|GetArrayItem` (`self.LevelNames`) (+ (`self.Get Current Level Index`) 1)))))

(fn `None Crystal Remaining`
  (returns (bool :type Boolean))
  (bind _outactors (`GameplayStatics.GetAllActorsOfClass` "/Game/BluePrints/Actors/BP_Crystal.BP_Crystal_C"))
  (return (== (`KismetArrayLibrary.Array_Length` _outactors) 0)))

(fn `Restart Game`
  (`GameplayStatics.OpenLevel` (`KismetStringLibrary.Conv_StringToName` (`|GetArrayItem` (`self.LevelNames`)))))

(fn `Set ContinueGame to False`
  (bind _returnvalue (`GameplayStatics.CreateSaveGameObject` "/Game/BluePrints/Actors/Volumes/BP_SaveGame.BP_SaveGame_C"))
  (set `/Game/BluePrints/Actors/Volumes/BP_SaveGame.Continue` false _returnvalue)
  (`GameplayStatics.SaveGameToSlot` _returnvalue "savegame"))

(fn `UserConstructionScript`)