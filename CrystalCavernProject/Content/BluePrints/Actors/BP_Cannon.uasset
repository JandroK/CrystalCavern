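; Cannon actor that spawns BP_Projectile at its Arrow, with a poof sound if recently rendered.
; BeginPlay starts a delayed firing loop unless ShootRate is 100; Tick also fires whenever CanShoot is set, apparently by a manager, and Shoot clears that flag.
; Each shot plays a Timeline that moves the cannon mesh along local Y, and its Fire event re-enters the ShootRate delay.
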(event `self.ReceiveBeginPlay`
  (bind _shoot_rate (`self.Shoot Rate`))
  ;[1 0.06419 0.09006] Shoot
  (if (!= _shoot_rate 100.0)
    (`KismetSystemLibrary.Delay` _shoot_rate :!label _label)
    (`self.Shoot` :!label _label_2)
    ;[1 0.7095 0.1876] Animation
    (bind (_direction _value) (`Timeline|Relative Cannon Location` :!via `PlayFromStart`)
      (:`Update`
        (`self.Set Cannon Location` _value))
      (:`Fire`
        (goto _label)))))

(event `self.ReceiveTick`
  (params (DeltaSeconds :type "Float (single-precision)"))
  ;[1 1 1] Can Shoot (From Manager)
  (if (`self.CanShoot`)
    (goto _label_2)))

(fn `Set Cannon Location`
  (params (NewLocation_Y :type "Float (double-precision)"))
  (`SceneComponent.K2_SetRelativeLocation` (`self.Cannon`) (`KismetMathLibrary.MakeVector` 0.0 NewLocation_Y) false false))

(fn `Shoot`
  (`|SpawnActorFromClass` "/Game/BluePrints/Actors/BP_Projectile.BP_Projectile_C" (`SceneComponent.K2_GetComponentToWorld` (`self.Arrow`)) "AlwaysSpawn" "OverrideRootScale" null null)
  (set `self.CanShoot` false)
  (if (`self.WasRecentlyRendered` 0.1)
    (`GameplayStatics.PlaySoundAtLocation` "/Game/Sounds/PoofEffect_Cue.PoofEffect_Cue" (`self.K2_GetActorLocation`) (struct) 1.0 1.0 0.0 null null null null)))

(fn `UserConstructionScript`)